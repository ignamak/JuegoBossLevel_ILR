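; BP_MagicWall is a trigger-activated barrier that appears when a character enters, marking the start of a battle.
; When a KGCharacterBase overlaps the Box while the Cube is hidden, the Cube becomes visible and collidable; the hidden check prevents retriggering once shown.
; It then finds BP_SoundManagerActor to play battle music and InGameHUD to dispatch the show-enemy-life event, both through GetAllActorsOfClass.
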(event OnComponentBeginOverlap(Box)
  (params (OverlappedComponent :type Primitive%20Component%20Object%20Reference) (OtherActor :type Actor%20Object%20Reference) (OtherComp :type Primitive%20Component%20Object%20Reference) (OtherBodyIndex :type Integer) (bFromSweep :type Boolean) (SweepResult :type Hit%20Result%20Structure%20%28by%20ref%29))
  (bind _cube (Variables|Default|GetCube))
  (if (Variables|/Script/Engine.SceneComponent|GetbHiddenInGame (Variables|Default|GetCube))
    (Utilities|Casting|CastToKGCharacterBase OtherActor)
    (Collision|SetCollisionEnabled _cube "QueryAndPhysics")
    (Development|SetHiddeninGame _cube false false)
    ;[1 1 1] Empieza musica batalla
    (bind _outactors (Actor|GetAllActorsOfClass "/Game/Sound/BP_SoundManagerActor.BP_SoundManagerActor_C"))
    (Default|PlayBattleMusic (Utilities|Array|Get(acopy) _outactors))
    ;[1 1 1] ShowLife
    (bind _outactors_2 (Actor|GetAllActorsOfClass "/Game/UI/InGameHUD.InGameHUD_C"))
    (Default|CallShowEnemyLifeEventDispatch (Variables|/Game/UI/InGameHUD.InGameHUD_C|GetPlayerInfoHUD_Ref (Utilities|Array|Get(acopy) _outactors_2)))))

(event EventBeginPlay)

(event Collision|EventActorBeginOverlap
  (params (OtherActor :type Actor%20Object%20Reference)))

(event EventTick
  (params (DeltaSeconds :type Float%20%28single-precision%29)))

(fn ConstructionScript)