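; Boss enemy character with melee, magic projectile and storm attacks, whose death triggers game over and victory music.
; Attack events play montages, apply damage through a sphere overlap at the right hand, spawn projectiles or attach storm actors.
; A looping timer checks health and tells the AI controller to change phase once at each of two thresholds.
; Damage triggers flinching, which blocks new attacks, or death, which also destroys the storms.
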(event Custom|EnemyMeleeAttack
  ;[1 1 1] MeleeAttack
  (if (not (Variables|Default|GetIsFlinching))
    (Animation|PlayAnimMontage "/Game/Assets/Enemy/EnemyAnims/Enemy_Attack_1_Montage.Enemy_Attack_1_Montage" 1.0 "None")))

(event Custom|EnemyTryDealMeleeDamage
  ;[1 1 1] MeleeDamage
  (bind (_outactors _returnvalue) (Collision|SphereOverlapActors (+ (Transformation|GetSocketLocation (Class|SkeletalMesh|FindSocket (Variables|/Script/Engine.SkinnedMeshComponent|GetSkeletalMesh (Variables|Character|GetMesh)) "hand_rSocket") (Variables|Character|GetMesh)) (* (Math|Vector|GetForwardVector (Variables|Default|GetArrow1)) 2e+01)) 1.5e+02 (Utilities|Array|MakeArray "ObjectTypeQuery3") "/Game/Blueprints/KnightBPs/KGCharacterBase.KGCharacterBase_C" (Utilities|Array|MakeArray self)))
  (if _returnvalue
    (Game|Damage|ApplyDamage (Utilities|Array|Get(acopy) _outactors) (Variables|Default|GetMeleeDamage) 0 self)))

(event Custom|AdvanceBossPhaseEvent
  (bind _self self)
  (bind _health (Variables|Default|GetHealth))
  (bind _returnvalue (Utilities|GetClass _self))
  (bind _health_2 (Utilities|GetClassDefaults _returnvalue))
  (bind _returnvalue_2 (/ _health _health_2))
  ;[1 1 1] CheckForPhaseSwitching
  (if (<= _returnvalue_2 (/ 3.0 5.0))
    (Utilities|FlowControl|Sequence
      (:then_0
        (Utilities|FlowControl|DoOnce false
          (:Completed
            (bind _asenemy_aicontroller (Utilities|Casting|CastToEnemyAIController (Pawn|GetController) :!label _label))
            (Default|ChangeBossPhaseEvent _asenemy_aicontroller))))
      (:then_1
        (if (<= _returnvalue_2 (/ 1.0 5.0))
          (Utilities|FlowControl|DoOnce false
            (:Completed
              (goto _label))))))))

(event Custom|EnemyLaunchProjectile
  ;[1 1 1] Magic
  (Game|SpawnActorfromClass "/Game/Blueprints/KGProjectileBase.KGProjectileBase_C" (Transformation|GetWorldTransform (Variables|Default|GetArrow1)) "Undefined" 0 self))

(event Custom|EnemyTryMagic
  ;[1 1 1] Magic
  (if (not (Variables|Default|GetIsFlinching))
    (Animation|PlayAnimMontage "/Game/Assets/Enemy/EnemyAnims/Enemy_Magic_Montage.Enemy_Magic_Montage" 1.0 "None")))

(event Custom|EnemyStartStorm
  (bind _self self)
  ;[1 1 1] Rayos Alrededor
  (for _index (range 0 5)
    (bind _returnvalue (Game|SpawnActorfromClass "/Game/Assets/Effects/StormAroundChar.StormAroundChar_C" (Transformation|GetActorTransform) "AlwaysSpawn" _self 0))
    (Utilities|Array|AddUnique (Variables|Default|GetStormRef) _returnvalue)
    (Transformation|AttachActorToActor _returnvalue _self (Transformation|GetAttachSocketName (Variables|Character|GetMesh _self)) "SnapToTarget" "KeepRelative" "KeepWorld" true)))

(event EventBeginPlay
  (bind _outactors (Actor|GetAllActorsOfClass "/Game/Sound/BP_SoundManagerActor.BP_SoundManagerActor_C"))
  (Variables|Default|SetSoundmanagerRef (Utilities|Array|Get(acopy) _outactors))
  (Utilities|Time|SetTimerbyEvent (delegate Custom|AdvanceBossPhaseEvent) 2.0 true))

(event Collision|EventActorBeginOverlap
  (params (OtherActor :type Actor%20Object%20Reference)))

(event EventTick
  (params (DeltaSeconds :type Float%20%28single-precision%29)))

(event Game|Damage|EventAnyDamage
  (params (Damage :type Float%20%28single-precision%29) (DamageType :type Damage%20Type%20Object%20Reference) (InstigatedBy :type Controller%20Object%20Reference) (DamageCauser :type Actor%20Object%20Reference))
  (bind _mesh (Variables|Character|GetMesh))
  (bind _soundmanagerref (Variables|Default|GetSoundmanagerRef))
  (bind _returnvalue (Components|SkeletalMesh|GetAnimInstance _mesh))
  ;[1 1 1] RecibirDaño
  (bind _output_get (Variables|Default|SetHealth (- (Variables|Default|GetHealth) Damage)))
  (if (<= _output_get 0.0)
    (Utilities|FlowControl|DoOnce false
      (:Completed
        ;;[1 1 1] Muerte
        (Variables|Default|SetisFlinching true)
        (Pawn|Components|CharacterMovement|DisableMovement (Variables|Character|GetCharacterMovement))
        (Utilities|FlowControl|Sequence
          (:then_0
            (bind _returnvalue_2 (Animation|PlayAnimMontage "/Game/Assets/Enemy/EnemyAnims/Enemy_Death_Montage.Enemy_Death_Montage" 1.0 "None"))
            (Utilities|FlowControl|Delay _returnvalue_2)
            (Actor|DestroyActor)
            (Default|GameOver (.AsKG%20Game%20Mode (Utilities|Casting|CastToKG_GameMode (Game|GetGameMode)))))
          (:then_1
            (for _array_element (Variables|Default|GetStormRef)
              (Utilities|IsValid _array_element
                (:Is%20Valid
                  (Actor|DestroyActor _array_element)))))
          (:then_2
            (Default|StopMusic _soundmanagerref)
            (Default|DeathSound _soundmanagerref self)
            (Utilities|FlowControl|Delay 0.2)
            (Default|VictoryMusic _soundmanagerref)))))
    (else
      (Utilities|FlowControl|Sequence
        (:then_0
          ;;[1 1 1] Flinch
          (Variables|Default|SetisFlinching true)
          (if (or (Class|AnimInstance|MontageIsActive _returnvalue "/Game/Assets/Enemy/EnemyAnims/Enemy_Attack_1_Montage.Enemy_Attack_1_Montage") (Class|AnimInstance|MontageIsActive _returnvalue "/Game/Assets/Enemy/EnemyAnims/Enemy_Magic_Montage.Enemy_Magic_Montage"))
            _
            (else
              (bind _returnvalue_3 (Animation|PlayAnimMontage "/Game/Assets/Enemy/EnemyAnims/Enemy_Flinch_Montage.Enemy_Flinch_Montage" 1.0 ""))
              (Utilities|FlowControl|Delay _returnvalue_3)))
          (Variables|Default|SetIsFlinching false))
        (:then_1
          (Default|ReceiveDamageGroaning (Variables|Default|GetSoundmanagerRef) self))))))

(fn ConstructionScript)