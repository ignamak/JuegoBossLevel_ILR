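; AI controller for enemies, including a boss with combat phases.
; On BeginPlay it runs the BT_Enemy behavior tree.
; A custom event increments the BossPhase counter and writes it to the BossPhaseBB blackboard key, so the behavior tree can read the current phase.
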(event Custom|ChangeBossPhaseEvent
  (bind _result (Math|Integer|IncrementInt (Variables|Default|GetBossPhase))
    (:%20%20
      (Class|BlackboardComponent|SetValueasInt (AI|GetBlackboard self) (Utilities|Name|MakeLiteralName "BossPhaseBB") _result))))

(event EventBeginPlay
  (AI|RunBehaviorTree "/Game/Blueprints/EnemyBPs/BT_Enemy.BT_Enemy"))

(fn ConstructionScript)