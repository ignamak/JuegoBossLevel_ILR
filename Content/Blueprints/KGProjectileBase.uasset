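; KGProjectileBase is a base projectile that damages player and enemy characters it overlaps.
; An overlap with a KGCharacterBase or EnemyCharacterBP other than its Instigator applies that target type's own damage value, then destroys the projectile.
; On destruction it spawns an impulse particle effect and applies a small radial damage burst at its location, credited to the Instigator's controller.
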(event EventBeginPlay)

(event Collision|EventActorBeginOverlap
  (params (OtherActor :type Actor%20Object%20Reference))
  (bind _instigator (Variables|Actor|GetInstigator))
  (bind _instigator_2 (Variables|Actor|GetInstigator))
  (bind _askgcharacter_base (Utilities|Casting|CastToKGCharacterBase OtherActor)
    (:then
      (if (not (== _askgcharacter_base _instigator_2))
        (Game|Damage|ApplyDamage _askgcharacter_base (Variables|Default|GetProjectileDamageToPlayer) (Pawn|GetController _instigator_2) self)
        (Actor|DestroyActor)))
    (:CastFailed
      (bind _asenemy_character_bp (Utilities|Casting|CastToEnemyCharacterBP OtherActor))
      (if (not (== _asenemy_character_bp _instigator))
        (Game|Damage|ApplyDamage _asenemy_character_bp (Variables|Default|GetProjectileDamageToEnemy) (Pawn|GetController _instigator) self)
        (Actor|DestroyActor)))))

(event EventTick
  (params (DeltaSeconds :type Float%20%28single-precision%29)))

(event EventDestroyed
  (bind _returnvalue (Transformation|GetActorLocation))
  (Effects|SpawnEmitteratLocation "/Game/Assets/Effects/PS_Impulse.PS_Impulse" _returnvalue)
  (Game|Damage|ApplyRadialDamage 2e+01 _returnvalue 5e+01 0 0 self (Pawn|GetController (Variables|Actor|GetInstigator)) false "ECC_Visibility"))

(fn ConstructionScript)