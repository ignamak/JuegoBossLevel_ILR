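; Player controller for a knight character that handles twin-stick style input, the HUD and pausing.
; Every tick it turns the pawn's yaw toward the cursor hit point, while movement follows the camera's up and right vectors.
; Attack inputs call melee, magic and auto-attack on KGCharacterBase, with auto-attack repeating on a timer while held.
; It plays a HUD pop-up on game mode new-wave events and toggles a pause menu.
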(event Custom|ProcessMouse
  (bind (_hitresult _returnvalue) (Game|Player|GetHitResultUnderCursorbyChannel "TraceTypeQuery1" true))
  (bind _returnvalue_2 (Pawn|GetControlledPawn))
  (bind _returnvalue_3 (Pawn|GetControlledPawn))
  (Utilities|IsValid _returnvalue_3
    (:Is%20Valid
      (bind _askgcharacter_base (Utilities|Casting|CastToKGCharacterBase _returnvalue_3))
      (if (and (> (Variables|/Game/Blueprints/KnightBPs/KGCharacterBase.KGCharacterBase_C|GetHealth _askgcharacter_base) 0.0) _returnvalue)
        (Transformation|SetActorRotation _returnvalue_2 (Math|Rotator|MakeRotator 0.0 0.0 (.yaw (Math|Conversions|RotationFromXVector (Math|Vector|GetUnitDirection(Vector) (Transformation|GetActorLocation _returnvalue_2) (.Location (Collision|BreakHitResult _hitresult)))))))))))

(event Custom|PopUpNewWaveUI
  (bind _uihudwidgetref (Variables|Default|GetUIHUDwidgetRef))
  (UserInterface|Animation|PlayAnimation _uihudwidgetref (Variables|/Game/UI/UI_HUD.UI_HUD_C|GetWaveCompletedPopUpAnim _uihudwidgetref) 0.0 1 "Forward" 1.0))

(event Custom|AutoAttackLoop
  ;[1 1 1] input attack
  (bind _askgcharacter_base (Utilities|Casting|CastToKGCharacterBase (Pawn|GetControlledPawn)))
  (Default|TryAutoAttack _askgcharacter_base))

(event EventBeginPlay
  (Variables|Default|SetbShowMouseCursor true)
  (bind _returnvalue (UserInterface|CreateWidget "/Game/UI/UI_HUD.UI_HUD_C"))
  (bind _output_get (Variables|Default|SetUIHUDwidgetRef _returnvalue))
  (UserInterface|Viewport|AddtoViewport _output_get 0)
  (bind _askg_game_mode (Utilities|Casting|CastToKG_GameMode (Game|GetGameMode)))
  (EventDispatchers|BindEventtoNewWave _askg_game_mode (delegate Custom|PopUpNewWaveUI)))

(event EventTick
  (params (DeltaSeconds :type Float%20%28single-precision%29))
  ;[1 1 1] NO
  (CallFunction|ProcessMouse))

(event Input|ActionEvents|InputActionJump
  (params (Key :type Key%20Structure))
  ;[1 1 1] input move
  (:Pressed
    (bind _ascharacter (Utilities|Casting|CastToCharacter (Pawn|GetControlledPawn)))
    (Character|Jump _ascharacter)))

(event Input|ActionEvents|InputActionMeleeAttack
  (params (Key :type Key%20Structure))
  ;[1 1 1] input attack
  (:Pressed
    (bind _askgcharacter_base (Utilities|Casting|CastToKGCharacterBase (Pawn|GetControlledPawn)))
    (Default|TryMelee _askgcharacter_base)))

(event Input|ActionEvents|InputActionMagicAttack
  (params (Key :type Key%20Structure))
  ;[1 1 1] input attack
  (:Pressed
    (bind _askgcharacter_base (Utilities|Casting|CastToKGCharacterBase (Pawn|GetControlledPawn)))
    (Default|TryMagic _askgcharacter_base)))

(event Input|ActionEvents|InputActionPause
  (params (Key :type Key%20Structure))
  ;[1 1 1] Pause
  (:Pressed
    (if (Game|IsGamePaused)
      (CallFunction|UnpauseGame)
      (else
        (CallFunction|PauseGame)))))

(event Input|ActionEvents|InputActionAutoAttack
  (params (Key :type Key%20Structure))
  ;[1 1 1] input attack
  (:Pressed
    (bind _returnvalue (Utilities|Time|SetTimerbyEvent (delegate Custom|AutoAttackLoop) 0.5 true)))
  (:Released
    (Utilities|Time|ClearandInvalidateTimerbyHandle _returnvalue)))

(event Input|AxisEvents|InputAxisUp
  (params (AxisValue :type Float%20%28single-precision%29))
  (bind _returnvalue (Pawn|GetControlledPawn))
  ;[1 1 1] input move
  (Utilities|IsValid _returnvalue
    (:Is%20Valid
      (Pawn|Input|AddMovementInput _returnvalue (Math|Vector|GetUpVector (Variables|/Script/Engine.PlayerCameraManager|GetTransformComponent (Variables|Default|GetPlayerCameraManager))) (* AxisValue 2.0) false))))

(event Input|AxisEvents|InputAxisRight
  (params (AxisValue :type Float%20%28single-precision%29))
  (bind _returnvalue (Pawn|GetControlledPawn))
  ;[1 1 1] input move
  (Utilities|IsValid _returnvalue
    (:Is%20Valid
      (Pawn|Input|AddMovementInput _returnvalue (Math|Vector|GetRightVector (Variables|/Script/Engine.PlayerCameraManager|GetTransformComponent (Variables|Default|GetPlayerCameraManager))) (* AxisValue 2.0) false))))

(fn ConstructionScript)

(fn PauseGame
  (Game|SetGamePaused true)
  (Utilities|IsValid (Variables|Default|GetPauseMenuWidgetRef)
    (:Is%20Valid
      _)
    (:Is%20Not%20Valid
      (bind _returnvalue (UserInterface|CreateWidget "/Game/UI/UI_PauseMenu.UI_PauseMenu_C" (Game|GetPlayerController 0)))
      (bind _output_get (Variables|Default|SetPauseMenuWidgetRef _returnvalue))))
  (UserInterface|Viewport|AddtoViewport _output_get 0))

(fn UnpauseGame
  (Game|SetGamePaused false)
  (Widget|RemovefromParent (Variables|Default|GetPauseMenuWidgetRef)))