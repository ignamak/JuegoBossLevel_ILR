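; Base knight character with sword melee, two projectile spells, damage reactions and death.
; BeginPlay attaches a sword and, for players only, starts timed magic recharge and caches the sound manager.
; Montages drive attacks and chaining; hits cause small or big flinches, except during AttackMoves sections.
; Player death triggers game over, other knights are destroyed, and living knights play a victory montage on the game-over dispatch.
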(event Custom|TryMagic
  ;[1 1 1] magic attack
  (if (and (not (Variables|Default|GetIsFlinching)) (>= (Variables|Default|GetStrongMagicValue) 50))
    (Animation|PlayAnimMontage "/Game/Assets/Knight/KnightAnims/MagicShootMontage.MagicShootMontage" 1.0 "None")))

(event Custom|TryAutoAttack
  ;[1 1 1] AutoAttack
  (if (and (not (Variables|Default|GetIsFlinching)) (> (Variables|Default|GetAutoMagicValue) 10))
    (Animation|PlayAnimMontage "/Game/Assets/Knight/KnightAnims/AutoShootMontage.AutoShootMontage" 1.0 "None")))

(event Custom|LaunchMagicProjectile
  ;[1 1 1] magic attack
  (Game|SpawnActorfromClass "/Game/Blueprints/KGProjectileBase.KGProjectileBase_C" (Transformation|GetWorldTransform (Variables|Default|GetArrow1)) "Undefined" 0 self)
  (Variables|Default|SetStrongMagicValue (- (Variables|Default|GetStrongMagicValue) 50)))

(event Custom|CreateSword
  ;[1 1 1] Spawn espada
  (bind _returnvalue (Game|SpawnActorfromClass "/Game/Blueprints/BaseSword.BaseSword_C" (Transformation|GetActorTransform) "Undefined" 0 0))
  (Transformation|AttachComponentToComponent _returnvalue (Variables|Character|GetMesh) "SwordSocket" "SnapToTarget" "SnapToTarget" "SnapToTarget" true)
  (Variables|Default|SetWeaponSwordRef _returnvalue))

(event Custom|UsePrimaryAttack
  ;[1 1 1] primary attack
  (CallFunction|TryMelee))

(event Custom|TryMelee
  (bind _mesh (Variables|Character|GetMesh))
  (bind _returnvalue (Components|SkeletalMesh|GetAnimInstance _mesh))
  (bind _returnvalue_2 (Animation|Montage|MontageGetCurrentSection _returnvalue "/Game/Assets/Knight/KnightAnims/KnightAttackMontage.KnightAttackMontage"))
  ;[1 1 1] melee attack
  (if (not (Variables|Default|GetIsFlinching))
    (if (Class|AnimInstance|MontageIsActive _returnvalue "/Game/Assets/Knight/KnightAnims/KnightAttackMontage.KnightAttackMontage")
      (switch name _returnvalue_2
        (:Attack1
          (Class|AnimInstance|MontageSetNextSection _returnvalue _returnvalue_2 "Attack2" "/Game/Assets/Knight/KnightAnims/KnightAttackMontage.KnightAttackMontage")))
      (else
        (Animation|PlayAnimMontage "/Game/Assets/Knight/KnightAnims/KnightAttackMontage.KnightAttackMontage" 1.0 "Attack1")))))

(event Custom|LaunchAutoProjectile
  ;[1 1 1] AutoAttack
  (Game|SpawnActorfromClass "/Game/Blueprints/KGProjectileAuto.KGProjectileAuto_C" (Transformation|GetWorldTransform (Variables|Default|GetArrow1)) "Undefined" 0 self)
  (Variables|Default|SetAutoMagicValue (- (Variables|Default|GetAutoMagicValue) 10)))

(event Custom|EndGameDance
  ;[1 1 1] GameOverAnim
  (if (> (Variables|Default|GetHealth) 0.0)
    (Pawn|Components|CharacterMovement|DisableMovement (Variables|Character|GetCharacterMovement))
    (Animation|PlayAnimMontage "/Game/Assets/Knight/KnightAnims/Victory_Montage.Victory_Montage" 1.0 "None")))

(event Custom|ChargeOverTimeMagic
  ;[1 1 1] ChargeMagic
  (Utilities|FlowControl|Sequence
    (:then_0
      (if (< (Variables|Default|GetStrongMagicValue) 100)
        (Variables|Default|SetStrongMagicValue (Math|Integer|Clamp(Integer) (+ (Variables|Default|GetStrongMagicValue) 2) 0 100))))
    (:then_1
      (if (< (Variables|Default|GetAutoMagicValue) 100)
        (Variables|Default|SetAutoMagicValue (Math|Integer|Clamp(Integer) (+ (Variables|Default|GetAutoMagicValue) 4) 0 100))))))

(event EventBeginPlay
  ;[1 1 1] BEGINPLAY
  (CallFunction|CreateSword)
  (bind _askg_game_mode (Utilities|Casting|CastToKG_GameMode (Game|GetGameMode)))
  (EventDispatchers|BindEventtoGameOverDispatch _askg_game_mode (delegate Custom|EndGameDance))
  (if (Pawn|IsPlayerControlled)
    (Utilities|Time|SetTimerbyEvent (delegate Custom|ChargeOverTimeMagic) 1.0 true)
    (bind _outactors (Actor|GetAllActorsOfClass "/Game/Sound/BP_SoundManagerActor.BP_SoundManagerActor_C"))
    (Variables|Default|SetSoundmanagerRef (Utilities|Array|Get(acopy) _outactors))))

(event Collision|EventActorBeginOverlap
  (params (OtherActor :type Actor%20Object%20Reference)))

(event EventTick
  (params (DeltaSeconds :type Float%20%28single-precision%29)))

(event Game|Damage|EventAnyDamage
  (params (Damage :type Float%20%28single-precision%29) (DamageType :type Damage%20Type%20Object%20Reference) (InstigatedBy :type Controller%20Object%20Reference) (DamageCauser :type Actor%20Object%20Reference))
  (bind _mesh (Variables|Character|GetMesh))
  (bind _soundmanagerref (Variables|Default|GetSoundmanagerRef))
  (bind _returnvalue (Components|SkeletalMesh|GetAnimInstance _mesh))
  ;[1 1 1] DAÑO
  ;;[1 1 1] Daño
  (bind _output_get (Variables|Default|SetHealth (- (Variables|Default|GetHealth) Damage)))
  (if (<= _output_get 0.0)
    (Utilities|FlowControl|DoOnce false
      (:Completed
        ;;[1 1 1] muerte
        (Utilities|FlowControl|Sequence
          (:then_0
            (Variables|Default|SetIsFlinching true)
            (Pawn|Components|CharacterMovement|DisableMovement (Variables|Character|GetCharacterMovement))
            (bind _returnvalue_2 (Animation|PlayAnimMontage "/Game/Assets/Knight/KnightAnims/KnightDeathMontage.KnightDeathMontage" 1.0 "None"))
            (if (Class|Controller|IsPlayerController (Pawn|GetController))
              ;;[1 1 1] Si el que muere es el jugador, gameover
              (Default|GameOver (.AsKG%20Game%20Mode (Utilities|Casting|CastToKG_GameMode (Game|GetGameMode))))
              (else
                (Utilities|FlowControl|Delay _returnvalue_2)
                (Actor|DestroyActor (Variables|Default|GetWeaponSwordRef))
                (Actor|DestroyActor))))
          (:then_1
            (Default|StopMusic _soundmanagerref)
            (Default|DeathSound _soundmanagerref self)
            (Utilities|FlowControl|Delay 0.2)
            (Default|DefeatMusic _soundmanagerref)))))
    (else
      (Utilities|FlowControl|Sequence
        (:then_0
          (Variables|Default|SetIsFlinching true)
          (if (Class|AnimInstance|MontageIsActive _returnvalue "/Game/Assets/Knight/KnightAnims/KnightAttackMontage.KnightAttackMontage")
            (if (Utilities|Array|ContainsItem (Variables|Default|GetAttackMoves) (Animation|Montage|MontageGetCurrentSection _returnvalue "/Game/Assets/Knight/KnightAnims/KnightAttackMontage.KnightAttackMontage"))
              (Variables|Default|SetIsFlinching false)
              (else
                ;;[1 1 1] Si te pilla recuperandote de un ataque, flinch grande
                (bind _returnvalue_3 (Animation|PlayAnimMontage "/Game/Assets/Knight/KnightAnims/PlayerFlinchMontage.PlayerFlinchMontage" 1.0 "FlinchBig"))
                (Utilities|FlowControl|Delay _returnvalue_3)
                (Variables|Default|SetIsFlinching false)))
            (else
              ;;[1 1 1] Si no está atacando, flinch pequeño
              (bind _returnvalue_4 (Animation|PlayAnimMontage "/Game/Assets/Knight/KnightAnims/PlayerFlinchMontage.PlayerFlinchMontage" 1.0 "FlinchSmall"))
              (Utilities|FlowControl|Delay _returnvalue_4)
              (Variables|Default|SetIsFlinching false))))
        (:then_1
          (Default|ReceiveDamageGroaning (Variables|Default|GetSoundmanagerRef) self))))))

(fn ConstructionScript
  (bind _returnvalue (Rendering|Material|CreateDynamicMaterialInstance (Variables|Character|GetMesh) 0 0 "None" :!class /Script/Engine.PrimitiveComponent))
  (Rendering|Material|SetVectorParameterValue _returnvalue "HairColour" (Variables|Default|GetHairColour) :!class /Script/Engine.MaterialInstanceDynamic))