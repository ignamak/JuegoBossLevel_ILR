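; KG_GameMode is a game mode with a game-over sequence and a disconnected, partly OLD-marked enemy wave system.
; GameOver fires a dispatcher, waits, blends the view to a random CameraActor, retrying those near the origin, then restarts the level.
; The legacy SpawnEnemy pops queued classes at random PlayerStarts and binds their destruction to a wave-completion check.
; Wave start and reset events are empty; their queue-shuffling logic and spawn timer never run.
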(event Custom|SpawnEnemy
  ;[1 0.071 0.04116] OLD
  (if (> (Utilities|Array|Length (Variables|Default|GetQueue)) 0)
    (bind _outactors (Actor|GetAllActorsOfClass "/Script/Engine.PlayerStart"))
    (bind _returnvalue (AI|SpawnAIFromClass (Utilities|Array|Get(acopy) (Variables|Default|GetQueue)) 0 (Transformation|GetActorLocation (Utilities|Array|Get(acopy) _outactors (Math|Random|RandomInteger (Utilities|Array|Length _outactors)))) (Transformation|GetActorRotation (Utilities|Array|Get(acopy) _outactors (Math|Random|RandomInteger (Utilities|Array|Length _outactors)))) false))
    ;;[1 1 1] Pop
    (Utilities|Array|RemoveIndex (Variables|Default|GetQueue))
    (Game|BindEventtoOnDestroyed _returnvalue (delegate Custom|CheckWaveCompleted))))

(event Custom|StartNewWave
  ;[1 0.01314 0] OLD
)

(event Custom|CheckWaveCompleted
  (params (DestroyedActor :type Actor%20Object%20Reference))
  ;[1 0.071 0.04116] OLD
  ;;[1 1 1] Si ya ha muerto la oleada anterior, spawn una nueva
  (if (== (Utilities|Array|Length (Variables|Default|GetQueue)) 0)
    (bind _outactors (Actor|GetAllActorsOfClass "/Game/Blueprints/KGAIControllerBase.KGAIControllerBase_C"))
    (if (== (Utilities|Array|Length _outactors) 0)
      (CallFunction|StartNewWave))))

(event Custom|ResetGameWaves
  ;[1 0.01314 0] OLD
)

(event Custom|GameOver
  ;[1 1 1] GAME OVER
  (Default|CallGameOverDispatch)
  ;[1 1 1] Tiempo para hacer la pose de victoria
  (Utilities|FlowControl|Delay 3.0)
  ;[1 1 1] Camerablend
  (bind _outactors (Actor|GetAllActorsOfClass "/Script/Engine.CameraActor" :!label _label))
  (bind _output_get (Variables|Default|SetCameraToBlendRef (Utilities|Array|Get(acopy) _outactors (Math|Random|RandomInteger (Utilities|Array|Length _outactors)))))
  (if (Math|Vector|Equal(Vector) (Transformation|GetActorLocation _output_get) "0, 0, 0" 1e+01)
    (goto _label)
    (else
      (Game|Player|SetViewTargetwithBlend (Game|GetPlayerController 0) _output_get 1.0 "VTBlend_Linear" 0.0 true)
      ;[1 1 1] Tras 3 seg, volver al menu
      (Utilities|FlowControl|Delay 3.0)
      (Development|ExecuteConsoleCommand "restartlevel" 0))))

(event EventBeginPlay)

(event EventTick
  (params (DeltaSeconds :type Float%20%28single-precision%29)))

(fn ConstructionScript)