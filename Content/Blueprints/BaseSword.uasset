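; Base sword actor that deals melee damage to enemy characters when its TryDealDamage event is called.
; The event runs a sphere overlap at the sword mesh for EnemyCharacterBP pawns, ignoring the owner of the component the sword is attached to.
; Each hit actor takes fixed damage and is passed to SwordHitFlesh on the sound manager actor, which is looked up with GetAllActorsOfClass on every hit.
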(event Custom|TryDealDamage
  (bind (_outactors _returnvalue) (Collision|SphereOverlapActors (Transformation|GetWorldLocation (Variables|Default|GetSwordMesh)) 1.2e+02 (Utilities|Array|MakeArray "ObjectTypeQuery3") "/Game/Blueprints/EnemyBPs/EnemyCharacterBP.EnemyCharacterBP_C" (Utilities|Array|MakeArray (Components|GetOwner (Transformation|GetAttachParent (Variables|Default|GetDefaultSceneRoot))))))
  (if _returnvalue
    (for _array_element _outactors
      (Game|Damage|ApplyDamage _array_element 3e+01 0 0)
      (bind _outactors_2 (Actor|GetAllActorsOfClass "/Game/Sound/BP_SoundManagerActor.BP_SoundManagerActor_C"))
      (Default|SwordHitFlesh (Utilities|Array|Get(acopy) _outactors_2) _array_element))))

(event EventBeginPlay)

(event Collision|EventActorBeginOverlap
  (params (OtherActor :type Actor%20Object%20Reference)))

(event EventTick
  (params (DeltaSeconds :type Float%20%28single-precision%29)))

(fn ConstructionScript)