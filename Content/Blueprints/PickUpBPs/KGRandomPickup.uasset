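; KGRandomPickup is a pickup actor that randomly becomes health, auto magic or strong magic on BeginPlay, with a matching sphere material.
; On overlap with a KGCharacterBase, it adds to that stat, capped at 100, unless the stat equals its class default, which is treated as full.
; A successful pickup destroys the actor and plays a sound through the first BP_SoundManagerActor found in the level.
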(event EventBeginPlay
  (bind _sphere1 (Variables|Default|GetSphere1))
  (switch int (Math|Random|RandomInteger 3)
    (:0
      (Variables|Default|SetPickUpEnum "NewEnumerator0")
      (Rendering|Material|SetMaterial _sphere1 0 "/Game/Materials/PickUpMaterial_Inst_Health.PickUpMaterial_Inst_Health"))
    (:1
      (Variables|Default|SetPickUpEnum "NewEnumerator2")
      (Rendering|Material|SetMaterial _sphere1 0 "/Game/Materials/PickUpMaterial_Inst_AutoMagic.PickUpMaterial_Inst_AutoMagic"))
    (:2
      (Variables|Default|SetPickUpEnum "NewEnumerator1")
      (Rendering|Material|SetMaterial _sphere1 0 "/Game/Materials/PickUpMaterial_Inst_StrongMagic.PickUpMaterial_Inst_StrongMagic"))))

(event Collision|EventActorBeginOverlap
  (params (OtherActor :type Actor%20Object%20Reference))
  (switch Utilities|FlowControl|Switch|SwitchonRandomPickUpEnum (Variables|Default|GetPickUpEnum)
    (:NewEnumerator0
      (bind _askgcharacter_base (Utilities|Casting|CastToKGCharacterBase OtherActor))
      (if (not (== (Variables|/Game/Blueprints/KnightBPs/KGCharacterBase.KGCharacterBase_C|GetHealth _askgcharacter_base) (.Health (Utilities|GetClassDefaults (Utilities|GetClass _askgcharacter_base)))))
        (Variables|/Game/Blueprints/KnightBPs/KGCharacterBase.KGCharacterBase_C|SetHealth _askgcharacter_base (Math|Float|Min(Float) (+ (Variables|/Game/Blueprints/KnightBPs/KGCharacterBase.KGCharacterBase_C|GetHealth _askgcharacter_base) (Variables|Default|GetHealthPickUpAmount)) 1e+02))
        (Actor|DestroyActor :!label _label)
        (bind _outactors (Actor|GetAllActorsOfClass "/Game/Sound/BP_SoundManagerActor.BP_SoundManagerActor_C"))
        (Default|PickupSFX (Utilities|Array|Get(acopy) _outactors))))
    (:NewEnumerator1
      (bind _askgcharacter_base_2 (Utilities|Casting|CastToKGCharacterBase OtherActor))
      (if (not (== (Variables|/Game/Blueprints/KnightBPs/KGCharacterBase.KGCharacterBase_C|GetStrongMagicValue _askgcharacter_base_2) (.StrongMagicValue (Utilities|GetClassDefaults (Utilities|GetClass _askgcharacter_base_2)))))
        (Variables|/Game/Blueprints/KnightBPs/KGCharacterBase.KGCharacterBase_C|SetStrongMagicValue _askgcharacter_base_2 (Math|Integer|Min(Integer) (+ (Variables|Default|GetStrongMagicPickUpAmount) (Variables|/Game/Blueprints/KnightBPs/KGCharacterBase.KGCharacterBase_C|GetStrongMagicValue _askgcharacter_base_2)) 100))
        (goto _label)))
    (:NewEnumerator2
      (bind _askgcharacter_base_3 (Utilities|Casting|CastToKGCharacterBase OtherActor))
      (if (not (== (Variables|/Game/Blueprints/KnightBPs/KGCharacterBase.KGCharacterBase_C|GetAutoMagicValue _askgcharacter_base_3) (.AutoMagicValue (Utilities|GetClassDefaults (Utilities|GetClass _askgcharacter_base_3)))))
        (Variables|/Game/Blueprints/KnightBPs/KGCharacterBase.KGCharacterBase_C|SetAutoMagicValue _askgcharacter_base_3 (Math|Integer|Min(Integer) (+ (Variables|Default|GetAutoMagicPickUpAmount) (Variables|/Game/Blueprints/KnightBPs/KGCharacterBase.KGCharacterBase_C|GetAutoMagicValue _askgcharacter_base_3)) 100))
        (goto _label)))))

(event EventTick
  (params (DeltaSeconds :type Float%20%28single-precision%29)))

(fn ConstructionScript)