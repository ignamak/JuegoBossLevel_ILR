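; BP_SoundManagerActor is a central sound manager actor that starts wildlife ambience on BeginPlay and exposes events for the game's music and effects.
; Pickup, victory and defeat play as 2D sounds, while battle music keeps a spawned component that StopMusic destroys.
; Sword hit, damage and death sounds attach to the given actor's root component.
; Damage and death cues randomize pitch, lower for EnemyCharacterBP and higher for other KGCharacterBase characters.
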(event Custom|SwordHitFlesh
  (params (Actor :type Actor%20Object%20Reference))
  ;[1 1 1] sword
  (Audio|SpawnSoundAttached "/Game/Sound/SFX/SwordHit/S_swordHit_CH_Cue.S_swordHit_CH_Cue" (Variables|/Script/Engine.Actor|GetRootComponent Actor) "None" "0, 0, 0" "0, 0, 0" "KeepRelativeOffset" false 1.0 1.0 0.0 0 0))

(event Custom|DeathSound
  (params (Actor :type Actor%20Object%20Reference))
  (bind _rootcomponent (Variables|/Script/Engine.Actor|GetRootComponent Actor))
  ;[1 1 1] damageDeath
  (Utilities|Casting|CastToEnemyCharacterBP Actor
    (:then
      (Audio|SpawnSoundAttached "/Game/Sound/SFX/Death/deathCH_Cue.deathCH_Cue" _rootcomponent "None" "0, 0, 0" "0, 0, 0" "KeepRelativeOffset" false 1.0 (Math|Random|RandomFloatinRange 0.6 0.8) 0.0 0 0))
    (:CastFailed
      (Utilities|Casting|CastToKGCharacterBase Actor)
      (Audio|SpawnSoundAttached "/Game/Sound/SFX/Death/deathCH_Cue.deathCH_Cue" _rootcomponent "None" "0, 0, 0" "0, 0, 0" "KeepRelativeOffset" false 1.0 (Math|Random|RandomFloatinRange 1.5 1.8) 0.0 0 0))))

(event Custom|ReceiveDamageGroaning
  (params (Actor :type Actor%20Object%20Reference))
  (bind _rootcomponent (Variables|/Script/Engine.Actor|GetRootComponent Actor))
  ;[1 1 1] damageDeath
  (Utilities|Casting|CastToEnemyCharacterBP Actor
    (:then
      (Audio|SpawnSoundAttached "/Game/Sound/SFX/CharReceiveDamage/receiveDamageCH_Cue.receiveDamageCH_Cue" _rootcomponent "None" "0, 0, 0" "0, 0, 0" "KeepRelativeOffset" false 1.0 (Math|Random|RandomFloatinRange 0.6 0.8) 0.0 0 0))
    (:CastFailed
      (Utilities|Casting|CastToKGCharacterBase Actor)
      (Audio|SpawnSoundAttached "/Game/Sound/SFX/CharReceiveDamage/receiveDamageCH_Cue.receiveDamageCH_Cue" _rootcomponent "None" "0, 0, 0" "0, 0, 0" "KeepRelativeOffset" false 1.0 (Math|Random|RandomFloatinRange 1.5 1.8) 0.0 0 0))))

(event Custom|PickupSFX
  ;[1 1 1] pickup
  (Audio|PlaySound2D "/Game/Sound/SFX/PickUp/PickUp_Cue.PickUp_Cue" 0.3 1.0 0.0 0 0))

(event Custom|VictoryMusic
  ;[1 1 1] gameover
  (Audio|PlaySound2D "/Game/Sound/Ambience/victory_Cue.victory_Cue" 1.0 1.0 0.0 0 0))

(event Custom|DefeatMusic
  ;[1 1 1] gameover
  (Audio|PlaySound2D "/Game/Sound/Ambience/defeat_Cue.defeat_Cue" 1.0 1.0 0.0 0 0))

(event Custom|PlayBattleMusic
  ;[1 1 1] ambience
  (bind _returnvalue (Audio|SpawnSound2D "/Game/Sound/Ambience/MusicBattle_Cue.MusicBattle_Cue" 0.5 1.0 0.0 0 false false)))

(event Custom|StopMusic
  (Components|DestroyComponent (stale Custom|PlayBattleMusic _returnvalue)))

(event EventBeginPlay
  ;[1 1 1] ambience
  (Audio|SpawnSound2D "/Game/Sound/Ambience/ambienceWildlife_Cue.ambienceWildlife_Cue" 0.5 1.0 0.0 0 false false))

(fn ConstructionScript)